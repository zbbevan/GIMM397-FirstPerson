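; Friendly quest-giver NPC that drives the dialogue, quest handout and win screen when talked to.
; Each Talkto shows the next line from one of three arrays, chosen by the player character's QuestGiven and QuestAmount, through a reused WB_Dialogue widget.
; Finishing the intro gives the quest; finishing the completion lines clears it, then shows WB_YouWin and pauses the game.
; Delays hold each final line before the dialogue closes.
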(event `/Game/FirstPerson/UI/BPI_Dialogue.TalkTo`
  (bind _returnvalue (`GameplayStatics.GetPlayerController` 0))
  (bind _completedtalkindex (`self.CompletedTalkIndex`))
  (bind _talkindex (`self.TalkIndex`))
  (bind _talkindex_2 (`self.TalkIndex`))
  (bind _asbp_first_person_character (cast `/Game/FirstPerson/Blueprints/BP_FirstPersonCharacter` (`GameplayStatics.GetPlayerCharacter` 0)))
  (if (`/Game/FirstPerson/Blueprints/BP_FirstPersonCharacter.QuestGiven` _asbp_first_person_character)
    (bind _asbp_first_person_character_2 (cast `/Game/FirstPerson/Blueprints/BP_FirstPersonCharacter` (`GameplayStatics.GetPlayerCharacter` 0)))
    (if (>= (`/Game/FirstPerson/Blueprints/BP_FirstPersonCharacter.QuestAmount` _asbp_first_person_character_2) 10)
      (`self.ContinueDialogue` (`|GetArrayItem` (`self.Dialogue3`) _completedtalkindex))
      (bind _result (`/Engine/EditorBlueprintResources/StandardMacros.IncrementInt` _completedtalkindex)
        (:`  `
          (if (== _result 3)
            (bind _asbp_first_person_character_3 (cast `/Game/FirstPerson/Blueprints/BP_FirstPersonCharacter` (`GameplayStatics.GetPlayerCharacter` 0)))
            (set `/Game/FirstPerson/Blueprints/BP_FirstPersonCharacter.QuestGiven` false _asbp_first_person_character_3)
            (`KismetSystemLibrary.Delay` 5.0)
            (bind _aswb_dialogue (cast `/Game/FirstPerson/UI/WB_Dialogue` (`self.DialogueUI`)))
            (`/Game/FirstPerson/UI/WB_Dialogue.CloseDialogue` _aswb_dialogue)
            (set `self.HasUI` false)
            (`KismetSystemLibrary.Delay` 5.0)
            (bind _returnvalue_2 (`|CreateWidget` "/Game/FirstPerson/UI/WB_YouWin.WB_YouWin_C" _returnvalue))
            (`UserWidget.AddToViewport` _returnvalue_2 0)
            (`GameplayStatics.SetGamePaused` true)
            (set `PlayerController.bShowMouseCursor` true _returnvalue))))
      (else
        (`self.ContinueDialogue` (`|GetArrayItem` (`self.Dialogue2`) _talkindex_2))
        (`/Engine/EditorBlueprintResources/StandardMacros.IncrementInt` _talkindex_2
          (:`  `
            (if (not (< (`self.TalkIndex`) (`KismetArrayLibrary.Array_Length` (`self.Dialogue2`))))
              (set `self.TalkIndex` 0)
              (`KismetSystemLibrary.Delay` 5.0)
              (bind _aswb_dialogue_2 (cast `/Game/FirstPerson/UI/WB_Dialogue` (`self.DialogueUI`)))
              (`/Game/FirstPerson/UI/WB_Dialogue.CloseDialogue` _aswb_dialogue_2)
              (set `self.HasUI` false))))))
    (else
      (`self.ContinueDialogue` (`|GetArrayItem` (`self.Dialogue1`) _talkindex))
      (`/Engine/EditorBlueprintResources/StandardMacros.IncrementInt` _talkindex
        (:`  `
          (if (not (< (`self.TalkIndex`) (`KismetArrayLibrary.Array_Length` (`self.Dialogue1`))))
            (bind _asbp_first_person_character_4 (cast `/Game/FirstPerson/Blueprints/BP_FirstPersonCharacter` (`GameplayStatics.GetPlayerCharacter` 0)))
            (set `/Game/FirstPerson/Blueprints/BP_FirstPersonCharacter.QuestGiven` true _asbp_first_person_character_4)
            (set `self.TalkIndex` 0)
            (`KismetSystemLibrary.Delay` 5.0)
            (bind _aswb_dialogue_3 (cast `/Game/FirstPerson/UI/WB_Dialogue` (`self.DialogueUI`)))
            (`/Game/FirstPerson/UI/WB_Dialogue.CloseDialogue` _aswb_dialogue_3)
            (set `self.HasUI` false)))))))

(event `ContinueDialogue`
  (params (TextToDisplay :type String))
  (if (not (`self.HasUI`))
    (bind _returnvalue (`|CreateWidget` "/Game/FirstPerson/UI/WB_Dialogue.WB_Dialogue_C" (`GameplayStatics.GetPlayerController` 0)))
    (bind _output_get (set `self.DialogueUI` _returnvalue))
    (`UserWidget.AddToViewport` _output_get 0)
    (set `self.HasUI` true))
  (`TextBlock.SetText` (`/Game/FirstPerson/UI/WB_Dialogue.TalkText` (`self.DialogueUI`)) (`KismetTextLibrary.Conv_StringToText` TextToDisplay)))

(fn `UserConstructionScript`)